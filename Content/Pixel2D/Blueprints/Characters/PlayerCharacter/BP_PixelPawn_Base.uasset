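; Base pawn for the Pixel2D player characters that can hand player control over to another pawn, its Target.
; Appear toggles the pawn's visibility and collision together.
; Persona! hides the current pawn, moves player 0's input and possession to a valid Target, reveals it, and quickly blends the camera view to it.
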(event `Appear`
  (params (`Show?` :type Boolean))
  (`self.SetActorHiddenInGame` (not `Show?`))
  (`self.SetActorEnableCollision` `Show?`)
  (if `Show?`
    _))

(event `Persona!`
  (bind _returnvalue (`GameplayStatics.GetPlayerController` 0))
  (bind _target (`self.Target`))
  (`self.Target`
    (:`then`
      (`self.Appear` false)
      (`Controller.UnPossess` _returnvalue)
      (`self.DisableInput` _returnvalue)
      (`self.EnableInput` _target _returnvalue)
      (`self.Appear` _target true)
      (`Controller.Possess` _returnvalue _target)
      (`PlayerController.SetViewTargetWithBlend` _returnvalue _target 0.1 "VTBlend_Linear" 0.0 false))
    (:`else`)))

(fn `UserConstructionScript`)