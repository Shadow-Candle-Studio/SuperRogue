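; BP_MeleeAttackZone is a short-lived box hit zone that applies melee damage to overlapping actors.
; On BeginPlay it takes damage and lifespan from its owner's BP_AttackComponent and sizes the box.
; Overlapping non-owner actors with a BP_HealthComponent lose health without knockback and show floating combat text.
; A ContinuousDamage option toggles an EnableDoT flag during overlap, but no damage-over-time logic appears here.
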(event `self.ReceiveBeginPlay`
  (bind _returnvalue (`self.GetComponentByClass` (`self.GetOwner`) "/Game/Public/Blueprints/BP_AttackComponent.BP_AttackComponent_C"))
  (`/Engine/EditorBlueprintResources/StandardMacros.IsValid` _returnvalue
    (:`Is Valid`
      (set `self.damage` (`/Game/Public/Blueprints/BP_AttackComponent.meleeDamage` _returnvalue))
      (set `self.ParentSceneComponent` (`/Game/Public/Blueprints/BP_AttackComponent.SceneComponent` _returnvalue))
      (bind _output_get (set `self.attackDuration` (`/Game/Public/Blueprints/BP_AttackComponent.attackDuration` _returnvalue)))
      (`self.SetLifeSpan` _output_get)
      (`BoxComponent.SetBoxExtent` (`self.Box`) (`KismetMathLibrary.MakeVector` (`self.boxWidth`) 100.0 (`self.boxHeight`)) true))))

(event `self.Box.OnComponentBeginOverlap`
  (params (OverlappedComponent :type "PrimitiveComponent Object Reference") (OtherActor :type "Actor Object Reference") (OtherComp :type "PrimitiveComponent Object Reference") (OtherBodyIndex :type Integer) (bFromSweep :type Boolean) (SweepResult :type "HitResult Structure (by ref)"))
  (bind _returnvalue (`self.GetComponentByClass` OtherActor "/Game/Public/Blueprints/BP_HealthComponent.BP_HealthComponent_C"))
  (bind _damage (`self.damage`))
  (`/Engine/EditorBlueprintResources/StandardMacros.IsValid` _returnvalue
    (:`Is Valid`
      (if (not (== OtherActor (`self.GetOwner`)))
        (`KismetSystemLibrary.PrintString` (`KismetStringLibrary.Conv_IntToString` _damage))
        (`/Game/Public/Blueprints/BP_HealthComponent.DecreaseHealth` _returnvalue _damage (0.0 0.0 0.0) null)
        (`/Game/Public/Blueprints/BP_CommonFunctions.SpawnFloatingCombatText` "NewEnumerator0" (`KismetTextLibrary.Conv_IntToText` _damage) "/Game/Public/Sprites/Final/S_Sword_Wooden.S_Sword_Wooden" (`self.K2_GetActorLocation` OtherActor))
        (if (`self.continuousDamage?`)
          (set `self.enableDoT` true))))))

(event `self.Box.OnComponentEndOverlap`
  (params (OverlappedComponent :type "PrimitiveComponent Object Reference") (OtherActor :type "Actor Object Reference") (OtherComp :type "PrimitiveComponent Object Reference") (OtherBodyIndex :type Integer))
  (set `self.enableDoT` false))

(event `self.ReceiveTick`
  (params (DeltaSeconds :type "Float (single-precision)")))

(fn `UserConstructionScript`)