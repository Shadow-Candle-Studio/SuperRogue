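; Energy potion item that restores a set amount of energy to the actor that uses it.
; On use it plays the use sound at the item's location, then calls RestoreEnergy on the owning actor with the item as instigator.
; Only when the restore succeeds does it decrease the stack by one and spawn a half-scale flipbook heal effect at the owner's X and Z position.
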(event `self.On Used`
  (params (OwningActor :type "Actor Object Reference"))
  (bind (_returnvalue_x _returnvalue_y _returnvalue_z) (`KismetMathLibrary.BreakVector` (`self.K2_GetActorLocation` OwningActor)))
  ;[1 1 1] Restores the specified amount of energy to the owner
  (`GameplayStatics.PlaySoundAtLocation` (`self.OnUseSound`) (`self.K2_GetActorLocation`) (struct) 1.0 1.0 0.0 null null null)
  (bind _success_ (`/Game/Public/Blueprints/BP_CommonFunctions.RestoreEnergy` OwningActor (`self.energyAmount`) false self))
  (if _success_
    (`self.DecreaseStack` 1)
    (`|SpawnActorFromClass` "/Game/Public/Blueprints/BP_Flipbook_FX.BP_Flipbook_FX_C" (`KismetMathLibrary.MakeTransform` (`KismetMathLibrary.MakeVector` _returnvalue_x 0.0 _returnvalue_z) (struct) (0.5 0.5 0.5)) "AlwaysSpawn" "OverrideRootScale" null "/Game/Public/FlipBooks/Final/FB_HealEffect.FB_HealEffect" false true null)))

(fn `UserConstructionScript`
  (`parent.UserConstructionScript`))