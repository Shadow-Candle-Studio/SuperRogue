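; Leveling component that tracks XP and level, responding to bound GrantXP and DecreaseXP events.
; AddXP runs CheckLevelUp, which scans PlayerXPTable thresholds (row count from ExperiencePTable), calls LevelUp per level gained, then spawns a flipbook effect at the owner.
; RemoveXP sets XP to the greater of the current level's threshold and Amount minus CurrentXP, never lowering the level.
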(event `self.ReceiveBeginPlay`
  (add `self.GrantXP` (delegate `GrantXP_Event`))
  (add `self.DecreaseXP` (delegate `DecreaseXP_Event`)))

(event `GrantXP_Event` :!signature `self.GrantXP`
  (params (Amount :type Integer) (SourceActor :type "Actor Object Reference"))
  (`self.AddXP` Amount))

(event `DecreaseXP_Event` :!signature `self.DecreaseXP`
  (params (Amount :type Integer) (SourceActor :type "Actor Object Reference"))
  (`self.RemoveXP` Amount))

(fn `AddXP`
  (params (Amount :type Integer))
  (bind _returnvalue_location (`KismetMathLibrary.BreakTransform` (`Actor.GetTransform` (`self.GetOwner`))))
  (set `self.currentXP` (+ Amount (`self.currentXP`)))
  (bind _levelsgained (`self.CheckLevelUp` (`self.currentLevel`)))
  (if (>= _levelsgained 1)
    (`|SpawnActorFromClass` "/Game/Public/Blueprints/BP_Flipbook_FX.BP_Flipbook_FX_C" (`KismetMathLibrary.MakeTransform` _returnvalue_location (struct) (0.2 0.2 0.2)) "AlwaysSpawn" "OverrideRootScale" null "/Game/Public/FlipBooks/Final/FB_level_up_102x136.FB_level_up_102x136" false true null)))

(fn `CheckLevelUp`
  (params (CurrentLevel :type Integer))
  (returns (LevelsGained :type Integer))
  (locals (tempLevel :type Integer) (` tempCur` :type Integer))
  (set `local. tempCur` CurrentLevel)
  (bind _outrownames (`DataTableFunctionLibrary.GetDataTableRowNames` (`self.experiencePTable`)))
  (for _index (range 1 (+ (+ (`KismetArrayLibrary.Array_LastIndex` _outrownames) 1) 1))
    (bind _returnvalue (`|GetDataTableRow` "/Game/Public/DataTable/PlayerXPTable.PlayerXPTable" (`KismetStringLibrary.Conv_StringToName` (`KismetTextLibrary.Conv_TextToString` (`KismetTextLibrary.Conv_IntToText` _index))))
      (:`then`
        (bind (_level _xprequired) (break `/Game/Public/Structure/ST_XPTableStructure` _returnvalue))
        (if (> _xprequired (`self.currentXP`))
          (set `local.tempLevel` _level)
          (break)))))
  (if (< (`local. tempCur`) (- (`local.tempLevel`) 1))
    (for _ (range 1 (+ (- (- (`local.tempLevel`) 1) (`local. tempCur`)) 1))
      (bind _result (`/Engine/EditorBlueprintResources/StandardMacros.IncrementInt` (`self.currentLevel`))
        (:`  `
          (`self.LevelUp` _result))))
    (return (- (`self.currentLevel`) (`local. tempCur`)))
    (else
      (return 0))))

(fn `GetCurrentLevel`
  (returns (Level :type Integer))
  (return (`self.currentLevel`)))

(fn `RemoveXP`
  (params (Amount :type Integer))
  (bind _returnvalue (`|GetDataTableRow` "/Game/Public/DataTable/PlayerXPTable.PlayerXPTable" (`KismetStringLibrary.Conv_StringToName` (`KismetStringLibrary.Conv_IntToString` (`self.currentLevel`))))
    (:`then`
      (set `self.currentXP` (`KismetMathLibrary.Max` (`.XPRequired_5_EC2262984EC426D2E5CDD6AE0496BE8A` (break `/Game/Public/Structure/ST_XPTableStructure` _returnvalue)) (- Amount (`self.currentXP`)))))))