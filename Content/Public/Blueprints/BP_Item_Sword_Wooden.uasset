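; Wooden sword item actor that performs a short melee attack for whoever uses it.
; On use it plays a sound at its location, then asks the owner's attack component for a melee trace from the HitSocket of its Pixel2D component, passing damage, knockback and the owner's enemy tag container.
; It sets a near-instant lifespan after attacking, and prints an error if either component is missing.
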(event `self.On Used`
  (params (OwningActor :type "Actor Object Reference"))
  (bind _returnvalue (`self.GetComponentByClass` OwningActor "/Game/Public/Blueprints/BP_AttackComponent.BP_AttackComponent_C"))
  (bind _returnvalue_2 (`self.GetComponentByClass` OwningActor "/Script/Pixel2D.Pixel2DComponent"))
  (bind _enemytags (message `/Game/Public/Blueprints/BP_GameplayTagInterface.GetEnemyTagContainer` OwningActor))
  (`GameplayStatics.PlaySoundAtLocation` (`self.OnUseSound`) (`self.K2_GetActorLocation`) (struct) 1.0 1.0 0.0 null null null)
  (`/Engine/EditorBlueprintResources/StandardMacros.IsValid` _returnvalue
    (:`Is Valid`
      (`/Engine/EditorBlueprintResources/StandardMacros.IsValid` _returnvalue_2
        (:`Is Valid`
          (`/Game/Public/Blueprints/BP_AttackComponent.MeleeTraceAttack` _returnvalue "HitSocket" _returnvalue_2 (`self.damage`) 0.3 (`self.attackSpeed`) 5.0 (struct :`R` 1.0 :`G` 1.0 :`B` 1.0 :`A` 1.0) (`self.knockbackForce`) _enemytags)
          (`self.SetLifeSpan` 0.01))
        (:`Is Not Valid`
          (`KismetSystemLibrary.PrintString` "Owner does not have a Pixel 2D component"))))
    (:`Is Not Valid`
      (`KismetSystemLibrary.PrintString` "Owner does not have Attack component"))))

(event `self.ReceiveBeginPlay`
  (`parent.ReceiveBeginPlay`))

(fn `GetEnemyTagContainer`
  (returns (EnemyTags :type "GameplayTagContainer Structure"))
  (return))

(fn `GetGameplayTagContainer`
  (returns (TagContainer :type "GameplayTagContainer Structure"))
  (return))

(fn `UserConstructionScript`
  (`parent.UserConstructionScript`))