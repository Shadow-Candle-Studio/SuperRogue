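; BP_DamageZone is a box trigger volume that damages and knocks back actors that have a BP_HealthComponent.
; On overlap it asks its DamageOnTouchComponent to deal damage, passing the actor's forward vector as the hit normal, and stops damage on end overlap.
; The construction script copies the zone's Damage and KnockbackForce settings into that component.
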(event `self.ReceiveBeginPlay`)

(event `self.Box.OnComponentBeginOverlap`
  (params (OverlappedComponent :type "PrimitiveComponent Object Reference") (OtherActor :type "Actor Object Reference") (OtherComp :type "PrimitiveComponent Object Reference") (OtherBodyIndex :type Integer) (bFromSweep :type Boolean) (SweepResult :type "HitResult Structure (by ref)"))
  (`/Engine/EditorBlueprintResources/StandardMacros.IsValid` (`self.GetComponentByClass` OtherActor "/Game/Public/Blueprints/BP_HealthComponent.BP_HealthComponent_C")
    (:`Is Valid`
      (`/Game/Public/Blueprints/BP_DamageOnTouchComponent.DealDamage` (`self.DamageOnTouchComponent`) OtherActor (`self.GetActorForwardVector` OtherActor)))))

(event `self.Box.OnComponentEndOverlap`
  (params (OverlappedComponent :type "PrimitiveComponent Object Reference") (OtherActor :type "Actor Object Reference") (OtherComp :type "PrimitiveComponent Object Reference") (OtherBodyIndex :type Integer))
  (`/Game/Public/Blueprints/BP_DamageOnTouchComponent.StopDealingDamage` (`self.DamageOnTouchComponent`) OtherActor))

(fn `UserConstructionScript`
  (bind _damageontouchcomponent (`self.DamageOnTouchComponent`))
  (set `/Game/Public/Blueprints/BP_DamageOnTouchComponent.damageAmount` (`self.damage`) _damageontouchcomponent)
  (set `/Game/Public/Blueprints/BP_DamageOnTouchComponent.knockbackForce` (`self.knockbackForce`) _damageontouchcomponent))