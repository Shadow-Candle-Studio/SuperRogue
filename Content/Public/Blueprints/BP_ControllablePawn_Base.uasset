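; Base controllable pawn that turns gamepad input into light-press and charge events and supports switching between characters.
; Each button runs a ProcessButton macro, using a timer at the key's boundary time to separate light press from charge.
; Per-key structs record times, state, event signs and trigger/stick axes, with CopySignsToAnim copying them between structs.
; Persona! hides this pawn, then reveals and possesses the target with a short camera blend.
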(event `Appear`
  (params (`Show?` :type Boolean))
  ;[1 1 1] Hide The player
  (`self.SetActorHiddenInGame` (not `Show?`))
  (`self.SetActorEnableCollision` `Show?`)
  (if `Show?`
    _))

(event `Persona!`
  (bind _returnvalue (`GameplayStatics.GetPlayerController` 0))
  (bind _target (`self.Target`))
  ;[1 1 1] CharacterChange
  (`self.Target`
    (:`then`
      (`self.Appear` false)
      (`Controller.UnPossess` _returnvalue)
      (`self.DisableInput` _returnvalue)
      (`self.EnableInput` _target _returnvalue)
      (`self.Appear` _target true)
      (`Controller.Possess` _returnvalue _target)
      (`PlayerController.SetViewTargetWithBlend` _returnvalue _target 0.1 "VTBlend_Linear" 0.0 false))
    (:`else`)))

(event `InputAction|LeftTrigger`
  (params (Key :type "Key Structure"))
  ;[1 1 1] LT and RT
  (:`Pressed`
    (bind _pressduration (`self.ProcessButton` (delegate `LTTransition`) (`self.LT`) :!label _label)
      (:`LightPressStartEvent`
        (`/Game/Public/Blueprints/BPI_InputReactionEvents.LightPressStartEvent_LT`))
      (:`LightPressOverEvent`
        (`/Game/Public/Blueprints/BPI_InputReactionEvents.LightPressOverEvent_LT` _pressduration))
      (:`ChargeStartEvent`
        (`/Game/Public/Blueprints/BPI_InputReactionEvents.ChargeStartEvent_LT`))
      (:`ChargeOverEvent`
        (`/Game/Public/Blueprints/BPI_InputReactionEvents.ChargeOverEvent_LT` _pressduration))))
  (:`Released`
    (goto _label :!via `ReleaseExe`)))

(event `InputAction|SpecialLeft`
  (params (Key :type "Key Structure"))
  ;[1 1 1] Special Button
  (:`Pressed`
    (bind _pressduration (`self.ProcessButton` (delegate `SpecialLeftTransition`) (`self.Special_L`) :!label _label_2)
      (:`LightPressStartEvent`
        (`/Game/Public/Blueprints/BPI_InputReactionEvents.SP_LightPressStartEvent_Left`))
      (:`LightPressOverEvent`
        (`/Game/Public/Blueprints/BPI_InputReactionEvents.SP_LightPressOverEvent_Left` _pressduration))
      (:`ChargeStartEvent`
        (`/Game/Public/Blueprints/BPI_InputReactionEvents.SP_ChargeStartEvent_Left`))
      (:`ChargeOverEvent`
        (`/Game/Public/Blueprints/BPI_InputReactionEvents.SP_ChargeOverEvent_Left` _pressduration))))
  (:`Released`
    (goto _label_2 :!via `ReleaseExe`)))

(event `LTTransition`
  ;[1 1 1] LT and RT
  (goto _label :!via `TimerEnterChargeAction`))

(event `SpecialLeftTransition`
  ;[1 1 1] Special Button
  (goto _label_2 :!via `TimerEnterChargeAction`))

(event `InputAction|LeftButtonGroup_left`
  (params (Key :type "Key Structure"))
  ;[1 1 1] LeftButtonGroup
  (:`Pressed`
    (bind _pressduration (`self.ProcessButton` (delegate `LBG_Transition_Left`) (`self.LBG_LEFT`) :!label _label_3)
      (:`LightPressStartEvent`
        (`/Game/Public/Blueprints/BPI_InputReactionEvents.LBG_LightPressStartEvent_Left`))
      (:`LightPressOverEvent`
        (`/Game/Public/Blueprints/BPI_InputReactionEvents.LBG_LightPressOverEvent_Left` 0.0))
      (:`ChargeStartEvent`
        (`/Game/Public/Blueprints/BPI_InputReactionEvents.LBG_ChargeStartEvent_Left`))
      (:`ChargeOverEvent`
        (`/Game/Public/Blueprints/BPI_InputReactionEvents.LBG_ChargeOverEvent_Left` _pressduration))))
  (:`Released`
    (goto _label_3 :!via `ReleaseExe`)))

(event `InputAction|RightButtonGroup_Left`
  (params (Key :type "Key Structure"))
  ;[1 1 1] RightbuttonGroup
  (:`Pressed`
    (bind _pressduration (`self.ProcessButton` (delegate `RBG_Transition_Left`) (`self.RBG_LEFT`) :!label _label_4)
      (:`LightPressStartEvent`
        (`/Game/Public/Blueprints/BPI_InputReactionEvents.RBG_LightPressStartEvent_Left`))
      (:`LightPressOverEvent`
        (`/Game/Public/Blueprints/BPI_InputReactionEvents.RBG_LightPressOverEvent_Left` _pressduration))
      (:`ChargeStartEvent`
        (`/Game/Public/Blueprints/BPI_InputReactionEvents.RBG_ChargeStartEvent_Left`))
      (:`ChargeOverEvent`
        (`/Game/Public/Blueprints/BPI_InputReactionEvents.RBG_ChargeOverEvent_Left` _pressduration))))
  (:`Released`
    (goto _label_4 :!via `ReleaseExe`)))

(event `InputAction|LeftShoulder`
  (params (Key :type "Key Structure"))
  ;[1 1 1] LB and RB
  (:`Pressed`
    (bind _pressduration (`self.ProcessButton` (delegate `LBTransition`) (`self.LB`) :!label _label_5)
      (:`LightPressStartEvent`
        (`/Game/Public/Blueprints/BPI_InputReactionEvents.LightPressStartEvent_LB`))
      (:`LightPressOverEvent`
        (`/Game/Public/Blueprints/BPI_InputReactionEvents.LightPressOverEvent_LB` _pressduration))
      (:`ChargeStartEvent`
        (`/Game/Public/Blueprints/BPI_InputReactionEvents.ChargeStartEvent_LB`))
      (:`ChargeOverEvent`
        (`/Game/Public/Blueprints/BPI_InputReactionEvents.ChargeOverEvent_LB` _pressduration))))
  (:`Released`
    (goto _label_5 :!via `ReleaseExe`)))

(event `LBG_Transition_Left`
  ;[1 1 1] LeftButtonGroup
  (goto _label_3 :!via `TimerEnterChargeAction`))

(event `RBG_Transition_Left`
  ;[1 1 1] RightbuttonGroup
  (goto _label_4 :!via `TimerEnterChargeAction`))

(event `InputAxis|LeftTriggerAxis`
  (params (AxisValue :type "Float (single-precision)"))
  ;[1 1 1] LT and RT
  (setmembers `/Game/Public/Structure/STR_InputKeyInfo` :`StructRef` (`self.LT`) :`AxisXValue` AxisValue))

(event `LBTransition`
  ;[1 1 1] LB and RB
  (goto _label_5 :!via `TimerEnterChargeAction`))

(event `InputAction|SpecialRight`
  (params (Key :type "Key Structure"))
  ;[1 1 1] Special Button
  (:`Pressed`
    (bind _pressduration (`self.ProcessButton` (delegate `SpecialRightTransition`) (`self.Special_R`) :!label _label_6)
      (:`LightPressStartEvent`
        (`/Game/Public/Blueprints/BPI_InputReactionEvents.SP_LightPressStartEvent_Right`))
      (:`LightPressOverEvent`
        (`/Game/Public/Blueprints/BPI_InputReactionEvents.SP_LightPressOverEvent_Right` _pressduration))
      (:`ChargeStartEvent`
        (`/Game/Public/Blueprints/BPI_InputReactionEvents.SP_ChargeStartEvent_Right`))
      (:`ChargeOverEvent`
        (`/Game/Public/Blueprints/BPI_InputReactionEvents.SP_ChargeOverEvent_Right` _pressduration))))
  (:`Released`
    (goto _label_6 :!via `ReleaseExe`)))

(event `InputAction|RightTrigger`
  (params (Key :type "Key Structure"))
  ;[1 1 1] LT and RT
  (:`Pressed`
    (bind _pressduration (`self.ProcessButton` (delegate `RTTransition`) (`self.RT`) :!label _label_7)
      (:`LightPressStartEvent`
        (`/Game/Public/Blueprints/BPI_InputReactionEvents.LightPressStartEvent_RT`))
      (:`LightPressOverEvent`
        (`/Game/Public/Blueprints/BPI_InputReactionEvents.LightPressOverEvent_RT` _pressduration))
      (:`ChargeStartEvent`
        (`/Game/Public/Blueprints/BPI_InputReactionEvents.ChargeStartEvent_RT`))
      (:`ChargeOverEvent`
        (`/Game/Public/Blueprints/BPI_InputReactionEvents.ChargeOverEvent_RT` _pressduration))))
  (:`Released`
    (goto _label_7 :!via `ReleaseExe`)))

(event `SpecialRightTransition`
  ;[1 1 1] Special Button
  (goto _label_6 :!via `TimerEnterChargeAction`))

(event `RTTransition`
  ;[1 1 1] LT and RT
  (goto _label_7 :!via `TimerEnterChargeAction`))

(event `InputAction|LeftButtonGroup_Right`
  (params (Key :type "Key Structure"))
  ;[1 1 1] LeftButtonGroup
  (:`Pressed`
    (bind _pressduration (`self.ProcessButton` (delegate `LBG_Transition_Right`) (`self.LBG_RIGHT`) :!label _label_8)
      (:`LightPressStartEvent`
        (`/Game/Public/Blueprints/BPI_InputReactionEvents.LBG_LightPressStartEvent_Right`))
      (:`LightPressOverEvent`
        (`/Game/Public/Blueprints/BPI_InputReactionEvents.LBG_LightPressOverEvent_Right` _pressduration))
      (:`ChargeStartEvent`
        (`/Game/Public/Blueprints/BPI_InputReactionEvents.LBG_ChargeStartEvent_Right`))
      (:`ChargeOverEvent`
        (`/Game/Public/Blueprints/BPI_InputReactionEvents.LBG_ChargeOverEvent_Right` _pressduration))))
  (:`Released`
    (goto _label_8 :!via `ReleaseExe`)))

(event `InputAction|RightbuttonGroup_Right`
  (params (Key :type "Key Structure"))
  ;[1 1 1] RightbuttonGroup
  (:`Pressed`
    (bind _pressduration (`self.ProcessButton` (delegate `RBG_Transition_Right`) (`self.RBG_RIGHT`) :!label _label_9)
      (:`LightPressStartEvent`
        (`/Game/Public/Blueprints/BPI_InputReactionEvents.RBG_LightPressStartEvent_Right`))
      (:`LightPressOverEvent`
        (`/Game/Public/Blueprints/BPI_InputReactionEvents.RBG_LightPressOverEvent_Right` _pressduration))
      (:`ChargeStartEvent`
        (`/Game/Public/Blueprints/BPI_InputReactionEvents.RBG_ChargeStartEvent_Right`))
      (:`ChargeOverEvent`
        (`/Game/Public/Blueprints/BPI_InputReactionEvents.RBG_ChargeOverEvent_Right` _pressduration))))
  (:`Released`
    (goto _label_9 :!via `ReleaseExe`)))

(event `InputAction|RightShoulder`
  (params (Key :type "Key Structure"))
  ;[1 1 1] LB and RB
  (:`Pressed`
    (bind _pressduration (`self.ProcessButton` (delegate `RBTransition`) (`self.RB`) :!label _label_10)
      (:`LightPressStartEvent`
        (`/Game/Public/Blueprints/BPI_InputReactionEvents.LightPressStartEvent_RB`))
      (:`LightPressOverEvent`
        (`/Game/Public/Blueprints/BPI_InputReactionEvents.LightPressOverEvent_RB` _pressduration))
      (:`ChargeStartEvent`
        (`/Game/Public/Blueprints/BPI_InputReactionEvents.ChargeStartEvent_RB`))
      (:`ChargeOverEvent`
        (`/Game/Public/Blueprints/BPI_InputReactionEvents.ChargeOverEvent_RB` _pressduration))))
  (:`Released`
    (goto _label_10 :!via `ReleaseExe`)))

(event `LBG_Transition_Right`
  ;[1 1 1] LeftButtonGroup
  (goto _label_8 :!via `TimerEnterChargeAction`))

(event `RBG_Transition_Right`
  ;[1 1 1] RightbuttonGroup
  (goto _label_9 :!via `TimerEnterChargeAction`))

(event `RBTransition`
  ;[1 1 1] LB and RB
  (goto _label_10 :!via `TimerEnterChargeAction`))

(event `InputAxis|RightTriggerAxis`
  (params (AxisValue :type "Float (single-precision)"))
  ;[1 1 1] LT and RT
  (setmembers `/Game/Public/Structure/STR_InputKeyInfo` :`StructRef` (`self.RT`) :`AxisXValue` AxisValue))

(event `InputAction|LeftButtonGroup_Up`
  (params (Key :type "Key Structure"))
  ;[1 1 1] LeftButtonGroup
  (:`Pressed`
    (bind _pressduration (`self.ProcessButton` (delegate `LBG_Transition_Up`) (`self.LBG_UP`) :!label _label_11)
      (:`LightPressStartEvent`
        (`/Game/Public/Blueprints/BPI_InputReactionEvents.LBG_LightPressStartEvent_Up`))
      (:`LightPressOverEvent`
        (`/Game/Public/Blueprints/BPI_InputReactionEvents.LBG_LightPressOverEvent_Up` _pressduration))
      (:`ChargeStartEvent`
        (`/Game/Public/Blueprints/BPI_InputReactionEvents.LBG_ChargeStartEvent_Up`))
      (:`ChargeOverEvent`
        (`/Game/Public/Blueprints/BPI_InputReactionEvents.LBG_ChargeOverEvent_Up` _pressduration))))
  (:`Released`
    (goto _label_11 :!via `ReleaseExe`)))

(event `InputAction|RightbuttonGroup_Up`
  (params (Key :type "Key Structure"))
  ;[1 1 1] RightbuttonGroup
  (:`Pressed`
    (bind _pressduration (`self.ProcessButton` (delegate `RBG_Transition_Top`) (`self.RBG_UP`) :!label _label_12)
      (:`LightPressStartEvent`
        (`/Game/Public/Blueprints/BPI_InputReactionEvents.RBG_LightPressStartEvent_Up`))
      (:`LightPressOverEvent`
        (`/Game/Public/Blueprints/BPI_InputReactionEvents.RBG_LightPressOverEvent_Up` _pressduration))
      (:`ChargeStartEvent`
        (`/Game/Public/Blueprints/BPI_InputReactionEvents.RBG_ChargeStartEvent_Up`))
      (:`ChargeOverEvent`
        (`/Game/Public/Blueprints/BPI_InputReactionEvents.RBG_ChargeOverEvent_Up` _pressduration))))
  (:`Released`
    (goto _label_12 :!via `ReleaseExe`)))

(event `InputAction|L3`
  (params (Key :type "Key Structure"))
  ;[1 1 1] LStick recording
  (:`Pressed`
    (bind _pressduration (`self.ProcessButton` (delegate `LStickEnterCharging`) (`self.LStick`) :!label _label_13)
      (:`LightPressStartEvent`
        (`/Game/Public/Blueprints/BPI_InputReactionEvents.LStickLightPressStartEvent`))
      (:`LightPressOverEvent`
        (`/Game/Public/Blueprints/BPI_InputReactionEvents.LStickLightPressOverEvent` _pressduration))
      (:`ChargeStartEvent`
        (`/Game/Public/Blueprints/BPI_InputReactionEvents.LStickChargeStartEvent`))
      (:`ChargeOverEvent`
        (`/Game/Public/Blueprints/BPI_InputReactionEvents.LStickChargeOverEvent` _pressduration))))
  (:`Released`
    (goto _label_13 :!via `ReleaseExe`)))

(event `LBG_Transition_Up`
  ;[1 1 1] LeftButtonGroup
  (goto _label_11 :!via `TimerEnterChargeAction`))

(event `RBG_Transition_Top`
  ;[1 1 1] RightbuttonGroup
  (goto _label_12 :!via `TimerEnterChargeAction`))

(event `InputAction|R3`
  (params (Key :type "Key Structure"))
  ;[1 1 1] RStick Recording
  (:`Pressed`
    (bind _pressduration (`self.ProcessButton` (delegate `RStickEnterCharging`) (`self.RStick`) :!label _label_14)
      (:`LightPressStartEvent`
        (`/Game/Public/Blueprints/BPI_InputReactionEvents.RStickLightPressStartEvent`))
      (:`LightPressOverEvent`
        (`/Game/Public/Blueprints/BPI_InputReactionEvents.RStickLightPressOverEvent` _pressduration))
      (:`ChargeStartEvent`
        (`/Game/Public/Blueprints/BPI_InputReactionEvents.RStickChargeStartEvent`))
      (:`ChargeOverEvent`
        (`/Game/Public/Blueprints/BPI_InputReactionEvents.RStickChargeOverEvent` _pressduration))))
  (:`Released`
    (goto _label_14 :!via `ReleaseExe`)))

(event `LStickEnterCharging`
  ;[1 1 1] LStick recording
  (goto _label_13 :!via `TimerEnterChargeAction`))

(event `RStickEnterCharging`
  ;[1 1 1] RStick Recording
  (goto _label_14 :!via `TimerEnterChargeAction`))

(event `InputAction|LeftButtonGroup_Down`
  (params (Key :type "Key Structure"))
  ;[1 1 1] LeftButtonGroup
  (:`Pressed`
    (bind _pressduration (`self.ProcessButton` (delegate `LBG_Transition_Down`) (`self.LBG_DOWN`) :!label _label_15)
      (:`LightPressStartEvent`
        (`/Game/Public/Blueprints/BPI_InputReactionEvents.LBG_LightPressStartEvent_Down`))
      (:`LightPressOverEvent`
        (`/Game/Public/Blueprints/BPI_InputReactionEvents.LBG_LightPressOverEvent_Down` _pressduration))
      (:`ChargeStartEvent`
        (`/Game/Public/Blueprints/BPI_InputReactionEvents.LBG_ChargeStartEvent_Down`))
      (:`ChargeOverEvent`
        (`/Game/Public/Blueprints/BPI_InputReactionEvents.LBG_ChargeOverEvent_Down` _pressduration))))
  (:`Released`
    (goto _label_15 :!via `ReleaseExe`)))

(event `InputAction|RightButtonGroup_Down`
  (params (Key :type "Key Structure"))
  ;[1 1 1] RightbuttonGroup
  (:`Pressed`
    (bind _pressduration (`self.ProcessButton` (delegate `RBG_Transition_Down`) (`self.RBG_DOWN`) :!label _label_16)
      (:`LightPressStartEvent`
        (`/Game/Public/Blueprints/BPI_InputReactionEvents.RBG_LightPressStartEvent_Down`))
      (:`LightPressOverEvent`
        (`/Game/Public/Blueprints/BPI_InputReactionEvents.RBG_LightPressOverEvent_Down` _pressduration))
      (:`ChargeStartEvent`
        (`/Game/Public/Blueprints/BPI_InputReactionEvents.RBG_ChargeStartEvent_Down`))
      (:`ChargeOverEvent`
        (`/Game/Public/Blueprints/BPI_InputReactionEvents.RBG_ChargeOverEvent_Down` _pressduration))))
  (:`Released`
    (goto _label_16 :!via `ReleaseExe`)))

(event `InputAxis|LeftThumbStickAxis_X`
  (params (AxisValue :type "Float (single-precision)"))
  ;[1 1 1] LStick recording
  (setmembers `/Game/Public/Structure/STR_InputKeyInfo` :`StructRef` (`self.LStick`) :`AxisXValue` AxisValue)
  (`/Game/Public/Blueprints/BPI_InputReactionEvents.LStickAxisEvent_X` AxisValue))

(event `InputAxis|RightThumbStickAxis_X`
  (params (AxisValue :type "Float (single-precision)"))
  ;[1 1 1] RStick Recording
  (setmembers `/Game/Public/Structure/STR_InputKeyInfo` :`StructRef` (`self.RStick`) :`AxisXValue` AxisValue)
  (`/Game/Public/Blueprints/BPI_InputReactionEvents.RStickAxisEvent_X` AxisValue))

(event `LBG_Transition_Down`
  ;[1 1 1] LeftButtonGroup
  (goto _label_15 :!via `TimerEnterChargeAction`))

(event `RBG_Transition_Down`
  ;[1 1 1] RightbuttonGroup
  (goto _label_16 :!via `TimerEnterChargeAction`))

(event `InputAxis|LeftThumbStickAxis_Y`
  (params (AxisValue :type "Float (single-precision)"))
  ;[1 1 1] LStick recording
  (setmembers `/Game/Public/Structure/STR_InputKeyInfo` :`StructRef` (`self.LStick`) :`AxisYValue` AxisValue)
  (`/Game/Public/Blueprints/BPI_InputReactionEvents.LStickAxisEvent_Y` AxisValue))

(event `InputAxis|RightThumbStickAxis_Y`
  (params (AxisValue :type "Float (single-precision)"))
  ;[1 1 1] RStick Recording
  (setmembers `/Game/Public/Structure/STR_InputKeyInfo` :`StructRef` (`self.RStick`) :`AxisYValue` AxisValue)
  (`/Game/Public/Blueprints/BPI_InputReactionEvents.RStickAxisEvent_Y` AxisValue))

(fn `Copy Signs to Anim`
  (params (Source :type "/Game/Public/Structure/STR_InputKeyInfo Structure (by ref)") (Dest :type "/Game/Public/Structure/STR_InputKeyInfo Structure (by ref)"))
  (bind (_lastpresstime _lastreleasetime _pressstate _is2daxis _axisxvalue _axisyvalue _lightpressstartsign _lightpressoversign _chargestartsign _chargeoversign _boundaryoflightandcharge) (break `/Game/Public/Structure/STR_InputKeyInfo` Source))
  (setmembers `/Game/Public/Structure/STR_InputKeyInfo` :`StructRef` Dest :`LastPressTime` _lastpresstime :`LastReleaseTime` _lastreleasetime :`PressState` _pressstate :`Is2DAxis` _is2daxis :`AxisXValue` _axisxvalue :`AxisYValue` _axisyvalue :`LightPressStartSign` _lightpressstartsign :`LightPressOverSign` _lightpressoversign :`ChargeStartSign` _chargestartsign :`ChargeOverSIgn` _chargeoversign :`BoundaryOfLightAndCharge` _boundaryoflightandcharge)
  (setmembers `/Game/Public/Structure/STR_InputKeyInfo` :`StructRef` Source :`LightPressStartSign` false :`LightPressOverSign` false :`ChargeStartSign` false :`ChargeOverSIgn` false))

(fn `UserConstructionScript`)