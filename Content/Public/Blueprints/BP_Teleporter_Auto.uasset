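; BP_Teleporter_Auto is a linked portal that automatically moves any actor entering its box to its ExitPortal.
; On overlap while active, it deactivates the exit portal to prevent bouncing back, then teleports the actor after a short delay, preserving its captured rotation.
; Expanding-circle flipbook effects appear at departure and arrival, with a sound at the entry portal.
; Each portal re-arms itself when an overlap with its box ends.
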(event `self.Box.OnComponentBeginOverlap`
  (params (OverlappedComponent :type "PrimitiveComponent Object Reference") (OtherActor :type "Actor Object Reference") (OtherComp :type "PrimitiveComponent Object Reference") (OtherBodyIndex :type Integer) (bFromSweep :type Boolean) (SweepResult :type "HitResult Structure (by ref)"))
  (bind _returnvalue_location (`KismetMathLibrary.BreakTransform` (`self.GetTransform` OtherActor)))
  (bind _exitportal (`self.exitPortal`))
  (bind _returnvalue_location_2 (`KismetMathLibrary.BreakTransform` (`self.GetTransform` _exitportal)))
  (if (`self.isActive?`)
    (set `/Game/Public/Blueprints/BP_Teleporter_Auto.isActive?` false (`self.exitPortal`))
    (set `self.localRotation` (`self.K2_GetActorRotation` OtherActor))
    (`KismetSystemLibrary.Delay` 0.2)
    (`|SpawnActorFromClass` "/Game/Public/Blueprints/BP_Flipbook_FX.BP_Flipbook_FX_C" (`KismetMathLibrary.MakeTransform` (+ _returnvalue_location (0.0 0.0 10.0)) (struct) (0.5 0.5 0.5)) "Undefined" "OverrideRootScale" null "/Game/Public/FlipBooks/Final/FB_ExpandCircle.FB_ExpandCircle" false true null)
    (`GameplayStatics.PlaySoundAtLocation` (`self.TeleportSound`) (`self.K2_GetActorLocation`) (struct) 2.0 1.0 0.0 null null null)
    (`self.K2_TeleportTo` OtherActor (`self.K2_GetActorLocation` _exitportal) (`self.localRotation`))
    (`|SpawnActorFromClass` "/Game/Public/Blueprints/BP_Flipbook_FX.BP_Flipbook_FX_C" (`KismetMathLibrary.MakeTransform` (+ _returnvalue_location_2 (0.0 0.0 10.0)) (struct) (0.5 0.5 0.5)) "Undefined" "OverrideRootScale" null "/Game/Public/FlipBooks/Final/FB_ExpandCircle.FB_ExpandCircle" false true null)))

(event `self.Box.OnComponentEndOverlap`
  (params (OverlappedComponent :type "PrimitiveComponent Object Reference") (OtherActor :type "Actor Object Reference") (OtherComp :type "PrimitiveComponent Object Reference") (OtherBodyIndex :type Integer))
  (set `self.isActive?` true))

(fn `UserConstructionScript`)