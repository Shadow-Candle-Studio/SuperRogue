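; BP_MapGeneration builds a randomized room-chain map at BeginPlay, running from a start piece through five links to a boss piece.
; Each Link call uses a random MultiGate to pick an LR, LRU or LRD piece, capping branching pieces with a Down or UP side piece.
; Pieces spawn at the origin, then move so their In point meets the previous Out point, which advances the chain.
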(event `self.ReceiveBeginPlay`
  (bind _returnvalue (`|SpawnActorFromClass` "/Game/Sprite/Tilemap/Actor_Map/BP_Start.BP_Start_C" (`KismetMathLibrary.MakeTransform` (0.0 0.0 0.0)) "AlwaysSpawn" "OverrideRootScale" null null))
  (set `self.OutLocation` (`SceneComponent.K2_GetComponentLocation` (`/Game/Sprite/Tilemap/Actor_Map/BP_MapParent.Out1` _returnvalue)))
  (while (< (stale _output_get) 5) :!label _label
    (`self.Link`)
    (bind _output_get (set `self.Count` (+ (`self.Count`) 1)))
    (goto _label))
  (bind _returnvalue_2 (`|SpawnActorFromClass` "/Game/Sprite/Tilemap/Actor_Map/BP_Boss.BP_Boss_C" (`KismetMathLibrary.MakeTransform` (0.0 0.0 0.0)) "AlwaysSpawn" "OverrideRootScale" null null))
  (`self.K2_SetActorLocation` _returnvalue_2 (- (`self.OutLocation`) (`SceneComponent.K2_GetComponentLocation` (`/Game/Sprite/Tilemap/Actor_Map/BP_MapParent.In` _returnvalue_2))) false false))

(fn `Link`
  (bind _returnvalue (`KismetMathLibrary.MakeTransform` (0.0 0.0 0.0)))
  (`|MultiGate` true
    (:`Out 0`
      (bind _returnvalue_2 (`|SpawnActorFromClass` "/Game/Sprite/Tilemap/Actor_Map/BP_LR.BP_LR_C" _returnvalue "Undefined" "OverrideRootScale" null null))
      (`self.K2_SetActorLocation` _returnvalue_2 (- (`self.OutLocation`) (`SceneComponent.K2_GetComponentLocation` (`/Game/Sprite/Tilemap/Actor_Map/BP_MapParent.In` _returnvalue_2))) false false)
      (set `self.OutLocation` (`SceneComponent.K2_GetComponentLocation` (`/Game/Sprite/Tilemap/Actor_Map/BP_MapParent.Out1` _returnvalue_2))))
    (:`Out 1`
      (bind _returnvalue_3 (`|SpawnActorFromClass` "/Game/Sprite/Tilemap/Actor_Map/BP_LRU.BP_LRU_C" _returnvalue "Undefined" "OverrideRootScale" null null))
      (`self.K2_SetActorLocation` _returnvalue_3 (- (`self.OutLocation`) (`SceneComponent.K2_GetComponentLocation` (`/Game/Sprite/Tilemap/Actor_Map/BP_MapParent.In` _returnvalue_3))) false false)
      (set `self.OutLocation` (`SceneComponent.K2_GetComponentLocation` (`/Game/Sprite/Tilemap/Actor_Map/BP_MapParent.Out1` _returnvalue_3)))
      (set `self.SideOutLocation` (`SceneComponent.K2_GetComponentLocation` (`/Game/Sprite/Tilemap/Actor_Map/BP_MapParent.Out2` _returnvalue_3)))
      (bind _returnvalue_4 (`|SpawnActorFromClass` "/Game/Sprite/Tilemap/Actor_Map/BP_Down.BP_Down_C" _returnvalue "Undefined" "OverrideRootScale" null null))
      (`self.K2_SetActorLocation` _returnvalue_4 (- (`self.SideOutLocation`) (`SceneComponent.K2_GetComponentLocation` (`/Game/Sprite/Tilemap/Actor_Map/BP_MapParent.In` _returnvalue_4))) false false))
    (:`Out 2`
      (bind _returnvalue_5 (`|SpawnActorFromClass` "/Game/Sprite/Tilemap/Actor_Map/BP_LRD.BP_LRD_C" _returnvalue "Undefined" "OverrideRootScale" null null))
      (`self.K2_SetActorLocation` _returnvalue_5 (- (`self.OutLocation`) (`SceneComponent.K2_GetComponentLocation` (`/Game/Sprite/Tilemap/Actor_Map/BP_MapParent.In` _returnvalue_5))) false false)
      (set `self.OutLocation` (`SceneComponent.K2_GetComponentLocation` (`/Game/Sprite/Tilemap/Actor_Map/BP_MapParent.Out1` _returnvalue_5)))
      (set `self.SideOutLocation` (`SceneComponent.K2_GetComponentLocation` (`/Game/Sprite/Tilemap/Actor_Map/BP_MapParent.Out2` _returnvalue_5)))
      (bind _returnvalue_6 (`|SpawnActorFromClass` "/Game/Sprite/Tilemap/Actor_Map/BP_UP.BP_UP_C" _returnvalue "Undefined" "OverrideRootScale" null null))
      (`self.K2_SetActorLocation` _returnvalue_6 (- (`self.SideOutLocation`) (`SceneComponent.K2_GetComponentLocation` (`/Game/Sprite/Tilemap/Actor_Map/BP_MapParent.In` _returnvalue_6))) false false))))

(fn `UserConstructionScript`)